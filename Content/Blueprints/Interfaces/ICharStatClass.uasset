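; ICharStatClass is a Blueprint interface for a single character stat with levels, experience and rust, declaring signatures with placeholder returns only.
; It exposes an enum name, progression queries, rust gain and loss rates, and functions to adjust level and XP.
; Wave-related functions cover base and current control, focus, amplitude, frequency and phase, plus a time-sampled stat wave.
; Further hooks handle refresh, level changes, influences and debug printing.
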(fn `DecBaseAmplitude`
  (params (`Decrease Amount` :type "Float (double-precision)"))
  (returns (`Base Amplitude` :type "Float (double-precision)"))
  (return 0.0))

(fn `DecBaseControl`
  (params (`Decrease Amount` :type Integer))
  (returns (`Base Control` :type Integer))
  (return 0))

(fn `DecBaseFocus`
  (params (`Decrease Amount` :type Integer))
  (returns (`Base Focus` :type Integer))
  (return 0))

(fn `DecBaseFrequency`
  (params (`Decrease Amount` :type "Float (double-precision)"))
  (returns (`Base Frequency` :type "Float (double-precision)"))
  (return 0.0))

(fn `DecBasePhase`
  (params (`Decrease Amount` :type "Float (double-precision)"))
  (returns (`Base Phase` :type "Float (double-precision)"))
  (return 0.0))

(fn `DecCurrentXP`
  (params (`Decrease Amount` :type Integer))
  (returns (`Current XP` :type Integer))
  (return 0))

(fn `DecStatLevel`
  (params (`Decrease Amount` :type Integer))
  (returns (Level :type Integer))
  (return 0))

(fn `Get All Info`
  (returns (`Stat Definition` :type "/Game/Blueprints/Data_Structures/Structs/Stats/StatDefinition Structure") (`Stat Controls` :type "/Game/Blueprints/Data_Structures/Structs/Stats/ControlStats Structure") (`Stat Wave Definitions` :type "/Game/Blueprints/Data_Structures/Structs/Stats/WaveDefinition Structure"))
  (return))

(fn `Get Base Amplitude`
  (returns (`Base Amplitude` :type "Float (double-precision)"))
  (return 0.0))

(fn `Get Base Focus`
  (returns (`Base Focus` :type Integer))
  (return 0))

(fn `Get Base Phase`
  (returns (`Base Phase` :type "Float (double-precision)"))
  (return 0.0))

(fn `Get Base Wave`
  (returns (Value :type "Float (double-precision)"))
  (return 0.0))

(fn `Get Current Amplitude`
  (returns (`Current Amplitude` :type "Float (double-precision)"))
  (return 0.0))

(fn `Get Current Control`
  (returns (`Current Control` :type "Float (double-precision)"))
  (return 0.0))

(fn `Get Current Focus`
  (returns (`Current Focus` :type "Float (double-precision)"))
  (return 0.0))

(fn `Get Current Frequency`
  (returns (`Current Frequency` :type "Float (double-precision)"))
  (return 0.0))

(fn `Get Current Phase`
  (returns (`Current Phase` :type "Float (double-precision)"))
  (return 0.0))

(fn `Get Level`
  (returns (`Current Level` :type Integer))
  (return 0))

(fn `Get MaxLevel`
  (returns (`Max Level` :type Integer))
  (return 0))

(fn `Get Name`
  (returns (Name :type "/Game/Blueprints/Data_Structures/Enums/MOBSpecific/EStats Enum"))
  (return "NewEnumerator0"))

(fn `GetBaseControl`
  (returns (`Base Control` :type Integer))
  (return 0))

(fn `GetBaseFrequency`
  (returns (`Base Frequency` :type "Float (double-precision)"))
  (return 0.0))

(fn `GetCurrentExperience`
  (returns (`Current Experience` :type Integer))
  (return 0))

(fn `GetExperienceGained`
  (returns (`Experienced Gained` :type Integer))
  (return 0))

(fn `GetExperienceToLevel`
  (returns (ExpToLevel :type Integer))
  (return 0))

(fn `GetHeighestLevelAchieved`
  (returns (`Highest Level` :type Integer))
  (return 0))

(fn `GetInfluences`
  (returns (`Influence Struct` :type "/Game/Blueprints/Data_Structures/Structs/Stats/StatInfluences Structure"))
  (return))

(fn `GetLowestRustLevel`
  (returns (`Lowest Rust Level` :type Integer))
  (return 0))

(fn `GetPercentageToLevel`
  (returns (`Percentage to Level` :type "Float (double-precision)"))
  (return 0.0))

(fn `GetPercentageToMaxLevel`
  (returns (`Percentage to Max` :type "Float (double-precision)"))
  (return 0.0))

(fn `GetRustGainRate`
  (returns (`Rust Gain Rate` :type "Float (double-precision)"))
  (return 0.0))

(fn `GetRustLossRate`
  (returns (`Rust Loss Rate` :type "Float (double-precision)"))
  (return 0.0))

(fn `GetStatWave`
  (params (Time :type Integer))
  (returns (Value :type "Float (double-precision)"))
  (return 0.0))

(fn `GetTotalExperiencedGained`
  (returns (`Total Experience Gained` :type Integer))
  (return 0))

(fn `IncBaseAmplitude`
  (params (`Increase Amount` :type "Float (double-precision)"))
  (returns (`Base Amplitude` :type "Float (double-precision)"))
  (return 0.0))

(fn `IncBaseControl`
  (params (`Increase Amount` :type Integer))
  (returns (`Base Control` :type Integer))
  (return 0))

(fn `IncBaseFocus`
  (params (`Increase amount` :type Integer))
  (returns (`Base Focus` :type Integer))
  (return 0))

(fn `IncBaseFrequency`
  (params (`Increase Amount` :type "Float (double-precision)"))
  (returns (`Base Frequency` :type "Float (double-precision)"))
  (return 0.0))

(fn `IncBasePhase`
  (params (`Increase Amount` :type "Float (double-precision)"))
  (returns (`Base Phase` :type "Float (double-precision)"))
  (return 0.0))

(fn `IncCurrentXP`
  (params (`Experince to Add` :type Integer))
  (returns (`Current XP` :type Integer))
  (return 0))

(fn `IncStatLevel`
  (params (`Amount to Increase` :type Integer))
  (returns (Level :type Integer))
  (return 0))

(fn `PrintStatControls`
  (returns (Return :type Boolean))
  (return false))

(fn `PrintStatDefinition`
  (returns (Return :type Boolean))
  (return false))

(fn `PrintStatWaveDef`
  (returns (Return :type Boolean))
  (return false))

(fn `Refresh Stat`)

(fn `StatLevelDown`)

(fn `StatLevelUp`)