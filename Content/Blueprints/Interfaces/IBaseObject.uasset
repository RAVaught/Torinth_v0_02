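; IBaseObject is a Blueprint interface that defines the common contract for game objects such as items.
; It declares name getters, inventory add, remove and destroy calls, and an inventory info query.
; A set of boolean action hooks covers moving, pickup, bagging, equipping, trading, examining, consuming and other item interactions.
; All functions are empty declarations with default returns, leaving behavior to the implementing classes.
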(fn `AddItemToInventory`)

(fn `Destroy Item`)

(fn `GetGetInventoryInfo`
  (returns (InventoryStruct :type "/Game/Blueprints/Data_Structures/Structs/Items/Item_Inventory_Struct Structure"))
  (return))

(fn `IF_GetName`
  (returns (Name :type Name))
  (return "None"))

(fn `IF_GetNameString`
  (returns (Name :type String))
  (return ""))

(fn `IOnBuy`
  (returns (NewParam :type Boolean))
  (return false))

(fn `IOnDestroy`
  (returns (NewParam :type Boolean))
  (return false))

(fn `IOnDrink`
  (returns (NewParam :type Boolean))
  (return false))

(fn `IOnEat`
  (returns (NewParam :type Boolean))
  (return false))

(fn `IOnExamine`
  (returns (NewParam :type Boolean))
  (return false))

(fn `IOnGive`
  (returns (NewParam :type Boolean))
  (return false))

(fn `IOnIdentify`
  (returns (NewParam :type Boolean))
  (return false))

(fn `IOnMove`
  (returns (NewParam :type Boolean))
  (return false))

(fn `IOnPickUp`
  (returns (NewParam :type Boolean))
  (return false))

(fn `IOnPutInBag`
  (returns (NewParam :type Boolean))
  (return false))

(fn `IOnSell`
  (returns (NewParam :type Boolean))
  (return false))

(fn `IOnSendToActionBar`
  (returns (NewParam :type Boolean))
  (return false))

(fn `IOnShowQuest`
  (returns (NewParam :type Boolean))
  (return false))

(fn `IOnTrade`
  (returns (NewParam :type Boolean))
  (return false))

(fn `IOnUse`
  (returns (NewParam :type Boolean))
  (return false))

(fn `IOnWear`
  (returns (NewParam :type Boolean))
  (return false))

(fn `IOnWield`
  (returns (NewParam :type Boolean))
  (return false))

(fn `Remove Item from Inventory`)