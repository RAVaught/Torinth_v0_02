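; ICharVitals is a Blueprint interface for a character's health, mana and fatigue vitals.
; It declares functions that modify each vital's current and maximum value by a passed amount, each returning a number.
; Getters expose each vital as a percent, and GetVitalsStruct serves as a query for the vitals struct.
; The functions hold no logic here, only signatures and default returns.
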(fn `GetFatiguePercent`
  (returns (FatiguePercent :type "Float (double-precision)"))
  (return 0.0))

(fn `GetHealthPercent`
  (returns (HPPercent :type "Float (double-precision)"))
  (return 0.0))

(fn `GetManaPercent`
  (returns (MPPercent :type "Float (double-precision)"))
  (return 0.0))

(fn `GetVitalsStruct`
  (returns (CharVitals :type "/Game/Blueprints/Data_Structures/Structs/Stats/CharVitals Structure"))
  (return))

(fn `ModifyCharFatigue`
  (params (FatigueToAdd :type "Float (double-precision)"))
  (returns (`New Value` :type "Float (double-precision)"))
  (return 0.0))

(fn `ModifyCharHealth`
  (params (HPToAdd :type "Float (double-precision)"))
  (returns (`new Value` :type "Float (double-precision)"))
  (return 0.0))

(fn `ModifyCharMana`
  (params (MPToAdd :type "Float (double-precision)"))
  (returns (`New Value` :type "Float (double-precision)"))
  (return 0.0))

(fn `ModifyCharMaxFatigue`
  (params (FatigueToAdd :type "Float (double-precision)"))
  (returns (`New Value` :type "Float (double-precision)"))
  (return 0.0))

(fn `ModifyCharMaxHealth`
  (params (MPToAdd :type "Float (double-precision)"))
  (returns (`New Value` :type "Float (double-precision)"))
  (return 0.0))

(fn `ModifyCharMaxMana`
  (params (ManaToDec :type "Float (double-precision)"))
  (returns (`New Value` :type "Float (double-precision)"))
  (return 0.0))