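; ICharStats is a Blueprint interface for reading and modifying character stats and awarding experience.
; Modifier functions take a stat and adjust its wave frequency, amplitude and phase, its level, control, focus and experience, or set prime, secondary and environmental influences and opposites.
; Getters expose eight attributes from Strength to Perception, a stat percentage, and stat wave queries with or without influences.
; It declares signatures only, leaving the logic to implementers.
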(fn `AwardEXP`
  (params (`Primary Stat` :type "/Game/Blueprints/Data_Structures/Enums/MOBSpecific/EStats Enum") (`Award Amount` :type Integer))
  (returns (Return :type Boolean))
  (return false))

(fn `Get Stat Wave`)

(fn `Get Stat Wave With Influences`
  (params (NewParam1 :type "/Game/Blueprints/Data_Structures/Enums/MOBSpecific/EStats Enum"))
  (returns (NewParam :type "Float (double-precision)"))
  (return 0.0))

(fn `IF_Get Agility`
  (returns (Agility :type Integer))
  (return 0))

(fn `IF_Get Charisma`
  (returns (Charisma :type Integer))
  (return 0))

(fn `IF_Get Constitution`
  (returns (Constitution :type Integer))
  (return 0))

(fn `IF_Get Dexterity`
  (returns (Dexterity :type Integer))
  (return 0))

(fn `IF_Get Intelligence`
  (returns (Intelligence :type Integer))
  (return 0))

(fn `IF_Get Perception`
  (returns (Perception :type Integer))
  (return 0))

(fn `IF_Get Strength`
  (returns (Strength :type Integer))
  (return 0))

(fn `IF_Get Wisdom`
  (returns (Wisdom :type Integer))
  (return 0))

(fn `IF_GetStatPercentage`
  (params (StatToGet :type "/Game/Blueprints/Data_Structures/Enums/MOBSpecific/EStats Enum"))
  (returns (`Percent to Max` :type "Float (double-precision)"))
  (return 0.0))

(fn `IF_ModBaseStatAmp`
  (params (`Stat To Mod` :type "/Game/Blueprints/Data_Structures/Enums/MOBSpecific/EStats Enum") (`Amp Adj` :type "Float (double-precision)"))
  (returns (`Adjusted Amp` :type "Float (double-precision)"))
  (return 0.0))

(fn `IF_ModBaseStatControl`
  (params (`Stat To Mod` :type "/Game/Blueprints/Data_Structures/Enums/MOBSpecific/EStats Enum") (`Adj Value` :type Integer))
  (returns (`Base Control` :type Integer))
  (return 0))

(fn `IF_ModBaseStatFocus`
  (params (`Stat To Mod` :type "/Game/Blueprints/Data_Structures/Enums/MOBSpecific/EStats Enum") (`Adj Value` :type Integer))
  (returns (`Base Focus` :type Integer))
  (return 0))

(fn `IF_ModBaseStatFreq`
  (params (`Stat To Mod` :type "/Game/Blueprints/Data_Structures/Enums/MOBSpecific/EStats Enum") (`Freq Adj` :type "Float (double-precision)"))
  (returns (`Adjusted Frequency` :type "Float (double-precision)"))
  (return 0.0))

(fn `IF_ModBaseStatLevel`
  (params (`Stat To Mod` :type "/Game/Blueprints/Data_Structures/Enums/MOBSpecific/EStats Enum") (`Adj Value` :type Integer))
  (returns (`Stat Level` :type Integer))
  (return 0))

(fn `IF_ModBaseStatPhase`
  (params (`Stat To Mod` :type "/Game/Blueprints/Data_Structures/Enums/MOBSpecific/EStats Enum") (`Phase Adj` :type "Float (double-precision)"))
  (returns (`Adjusted Phase` :type "Float (double-precision)"))
  (return 0.0))

(fn `IF_ModEnvInfluence`
  (params (`Stat To Mod` :type "/Game/Blueprints/Data_Structures/Enums/MOBSpecific/EStats Enum") (`New Influence` :type "/Game/Blueprints/Data_Structures/Enums/GenericInfo/EEnvInfluences Enum"))
  (returns (`Updated Influence` :type "/Game/Blueprints/Data_Structures/Enums/GenericInfo/EEnvInfluences Enum"))
  (return "NewEnumerator0"))

(fn `IF_ModEnvOpposite`
  (params (`Stat To Mod` :type "/Game/Blueprints/Data_Structures/Enums/MOBSpecific/EStats Enum") (`New Opposite` :type "/Game/Blueprints/Data_Structures/Enums/GenericInfo/EEnvInfluences Enum"))
  (returns (`Updated Influence` :type "/Game/Blueprints/Data_Structures/Enums/GenericInfo/EEnvInfluences Enum"))
  (return "NewEnumerator0"))

(fn `IF_ModPrimeInfluence`
  (params (`Stat To Mod` :type "/Game/Blueprints/Data_Structures/Enums/MOBSpecific/EStats Enum") (NewInfluence :type "/Game/Blueprints/Data_Structures/Enums/MOBSpecific/EStats Enum"))
  (returns (`Updated Influence` :type "/Game/Blueprints/Data_Structures/Enums/MOBSpecific/EStats Enum"))
  (return "NewEnumerator0"))

(fn `IF_ModPrimeOpposite`
  (params (`Stat To Mod` :type "/Game/Blueprints/Data_Structures/Enums/MOBSpecific/EStats Enum") (NewOpposite :type "/Game/Blueprints/Data_Structures/Enums/MOBSpecific/EStats Enum"))
  (returns (`Updated Opposite` :type "/Game/Blueprints/Data_Structures/Enums/MOBSpecific/EStats Enum"))
  (return "NewEnumerator0"))

(fn `IF_ModSecondaryInfluence`
  (params (`Stat To Mod` :type "/Game/Blueprints/Data_Structures/Enums/MOBSpecific/EStats Enum") (NewInfluence :type "/Game/Blueprints/Data_Structures/Enums/MOBSpecific/EStats Enum"))
  (returns (`Updated Influence` :type "/Game/Blueprints/Data_Structures/Enums/MOBSpecific/EStats Enum"))
  (return "NewEnumerator0"))

(fn `IF_ModSecondaryOpposite`
  (params (`Stat To Mod` :type "/Game/Blueprints/Data_Structures/Enums/MOBSpecific/EStats Enum") (NewOpposite :type "/Game/Blueprints/Data_Structures/Enums/MOBSpecific/EStats Enum"))
  (returns (`Updated Opposite` :type "/Game/Blueprints/Data_Structures/Enums/MOBSpecific/EStats Enum"))
  (return "NewEnumerator0"))

(fn `IF_ModStatExp`
  (params (`Stat To Mod` :type "/Game/Blueprints/Data_Structures/Enums/MOBSpecific/EStats Enum") (`Mod Amount` :type Integer))
  (returns (`Current XP` :type Integer))
  (return 0))