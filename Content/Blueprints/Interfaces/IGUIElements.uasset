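; IGUIElements is a Blueprint interface that declares the calls for controlling GUI elements.
; Its functions send a menu array with a target object, show the context menu, close a given widget, toggle the character and inventory screens, and create the default UI.
; It holds only signatures with stub returns, so the behavior comes from whichever class implements it.
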(fn `CloseWidget`
  (params (`Widget To Close` :type "Widget Object Reference"))
  (returns (Return :type Boolean))
  (return false))

(fn `CreateDefaultUI`
  (returns (NewParam :type Boolean))
  (return false))

(fn `Send Context Menu`
  (params (MenuArray :type "Array of /Game/Blueprints/GameInfo/Enums/MenuItems/EContextMenu Enum") (`Target Object` :type "Actor Object Reference"))
  (returns (Return :type Boolean))
  (return false))

(fn `ShowContextMenu`
  (returns (Return :type Boolean))
  (return false))

(fn `ToggleCharacterScreen`
  (returns (NewParam :type Boolean))
  (return false))

(fn `ToggleInventoryScreen`
  (returns (NewParam :type Boolean))
  (return false))