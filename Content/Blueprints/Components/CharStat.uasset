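; Character stat component that stores RPG attributes (Strength through Perception) in a struct array, with per-stat experience and leveling.
; AwardEXP scales awards by gain rate and loops through level-ups, carrying over excess XP.
; CalcXpToLevel intends gap-based costs, but divides by literal 0 or 1.
; Interface functions read scores and adjust wave-like stat fields with limits or wrapping; ModStatControl writes Focus, ModStatFreq reads Amplitude, and ModStatScore is a stub.
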(event EventTick
  (params (DeltaSeconds :type Float%20%28single-precision%29)))

(event EventInitializeComponent)

(fn FindStat
  (params (StatName :type EStats%20Enum :default "NewEnumerator0"))
  (return (Utilities|Array|Get(acopy) (Variables|Default|GetStats) (Utilities|Array|FindItem (Variables|Default|GetStats) (Utilities|Struct|MakeCharStatsV2 StatName 0 0 0.0)))))

(fn CheckEXPGains
  (params (Current :type Integer :default 0) (Max :type Integer :default 0))
  ;[1 1 1] Check if the current Amount is greater than the max needed to level
  (bind _output_get (LocalVariables|SetGainedLevel (>= Current Max)))
  (if _output_get
    (LocalVariables|SetTempXpVal (- Current Max))
    (else
      (LocalVariables|SetTempXpVal Current)))
  (return (LocalVariables|GetGainedLevel) (LocalVariables|GetTempXpVal)))

(fn CalcXptoLevel
  (params (StatScore :type Integer :default 0))
  (bind _returnvalue (* StatScore 5))
  ;[1 1 1] Calc the sum of all stat scores
  (for _array_element (Variables|Default|GetStats)
    (LocalVariables|SetLevelSum (+ (.Score (Utilities|Struct|BreakCharStatsV2 _array_element)) (LocalVariables|GetLevelSum)))
    (if (> (.Score (Utilities|Struct|BreakCharStatsV2 _array_element)) (LocalVariables|GetHighestScore))
      (LocalVariables|SetHighestScore (.Score (Utilities|Struct|BreakCharStatsV2 _array_element)))))
  ;[1 1 1] The xp needed to level is the (Score * 5)(Sum of all levels/difference between the current score and the highest score). The larger the gap the less XP is needed to level. This also scales with total experience earned, so that higher level players will pay more for building up lower level stats.
  (if (!= (- (LocalVariables|GetHighestScore) StatScore) 0)
    (LocalVariables|SetToLevel (* _returnvalue (/ (LocalVariables|GetLevelSum) 0)))
    (else
      (LocalVariables|SetToLevel (* _returnvalue (/ (LocalVariables|GetLevelSum) 1)))))
  (return (LocalVariables|GetToLevel)))

(fn LevelStat
  (params (StatToLevel :type EStats%20Enum :default "NewEnumerator0"))
  (bind _statstruct (CallFunction|FindStat StatToLevel))
  (Utilities|Struct|SetmembersinCharStatsV2 _statstruct (+ (.Score (Utilities|Struct|BreakCharStatsV2 _statstruct)) 1))
  (bind _xptolevel (CallFunction|CalcXptoLevel (.Score (Utilities|Struct|BreakCharStatsV2 _statstruct))))
  (Utilities|Struct|SetmembersinCharStatsV2 _statstruct _xptolevel))

(fn AwardEXP
  (params (StatToAward :type EStats%20Enum :default "NewEnumerator0") (Award%20Amount :type Integer))
  (bind _statstruct (CallFunction|FindStat StatToAward))
  (bind (_levelgained _currentxpvalue) (CallFunction|CheckEXPGains (+ (Math|Float|Round (* Award%20Amount (.ExperienceGainRate (Utilities|Struct|BreakCharStatsV2 _statstruct)))) (.Experience (Utilities|Struct|BreakCharStatsV2 _statstruct))) (.ExperienceToLevel (Utilities|Struct|BreakCharStatsV2 _statstruct)) :!label _label))
  (bind _output_get (LocalVariables|SetGained _levelgained))
  (if _output_get
    (bind _xptolevel (CallFunction|CalcXptoLevel (+ (.Score (Utilities|Struct|BreakCharStatsV2 _statstruct)) 1)))
    (Utilities|Struct|SetmembersinCharStatsV2 _statstruct _currentxpvalue _xptolevel)
    (CallFunction|LevelStat (.StatEnum (Utilities|Struct|BreakCharStatsV2 _statstruct)))
    (goto _label)
    (else
      (Utilities|Struct|SetmembersinCharStatsV2 _statstruct _currentxpvalue)
      (return (LocalVariables|GetCompleted)))))

(fn IFGetAgility
  (bind _statstruct (CallFunction|FindStat "NewEnumerator3"))
  (return (.Score (Utilities|Struct|BreakCharStatsV2 _statstruct))))

(fn IFGetCharisma
  (bind _statstruct (CallFunction|FindStat "NewEnumerator6"))
  (return (.Score (Utilities|Struct|BreakCharStatsV2 _statstruct))))

(fn IFGetConstitution
  (bind _statstruct (CallFunction|FindStat "NewEnumerator1"))
  (return (.Score (Utilities|Struct|BreakCharStatsV2 _statstruct))))

(fn IFGetDexterity
  (bind _statstruct (CallFunction|FindStat "NewEnumerator2"))
  (return (.Score (Utilities|Struct|BreakCharStatsV2 _statstruct))))

(fn IFGetIntelligence
  (bind _statstruct (CallFunction|FindStat "NewEnumerator5"))
  (return (.Score (Utilities|Struct|BreakCharStatsV2 _statstruct))))

(fn IFGetPerception
  (bind _statstruct (CallFunction|FindStat "NewEnumerator7"))
  (return (.Score (Utilities|Struct|BreakCharStatsV2 _statstruct))))

(fn IFGetStrength
  (bind _statstruct (CallFunction|FindStat "NewEnumerator0"))
  (return (.Score (Utilities|Struct|BreakCharStatsV2 _statstruct))))

(fn IFGetWisdom
  (bind _statstruct (CallFunction|FindStat "NewEnumerator4"))
  (return (.Score (Utilities|Struct|BreakCharStatsV2 _statstruct))))

(fn IFGetStatPercentage
  (params (StatToGet :type EStats%20Enum :default "NewEnumerator0"))
  (bind _statstruct (CallFunction|FindStat StatToGet))
  (return (/ (Math|Conversions|ToFloat(Integer) (.Experience (Utilities|Struct|BreakCharStatsV2 _statstruct))) (Math|Conversions|ToFloat(Integer) (Variables|Default|GetStatMax)))))

(fn IFModStatAmp
  (params (Stat%20To%20Mod :type EStats%20Enum :default "NewEnumerator0") (Amp%20Adj :type Float%20%28single-precision%29))
  (bind _statstruct (CallFunction|FindStat Stat%20To%20Mod))
  (if (and (<= (+ (.Amplitude (Utilities|Struct|BreakCharStatsV2 _statstruct)) Amp%20Adj) (Math|Conversions|ToFloat(Integer) (* (.Score (Utilities|Struct|BreakCharStatsV2 _statstruct)) (Variables|Default|GetAmplitudeMultiplier)))) (> (+ (.Amplitude (Utilities|Struct|BreakCharStatsV2 _statstruct)) Amp%20Adj) 0.0))
    (Utilities|Struct|SetmembersinCharStatsV2 _statstruct (+ (.Amplitude (Utilities|Struct|BreakCharStatsV2 _statstruct)) Amp%20Adj))
    (elif (> (+ (.Amplitude (Utilities|Struct|BreakCharStatsV2 _statstruct)) Amp%20Adj) 0.0)
      (Utilities|Struct|SetmembersinCharStatsV2 _statstruct (Math|Conversions|ToFloat(Integer) (* (.Score (Utilities|Struct|BreakCharStatsV2 _statstruct)) (Variables|Default|GetAmplitudeMultiplier))))
      (else
        (Utilities|Struct|SetmembersinCharStatsV2 _statstruct 1.0))))
  (return 0.0))

(fn IFModStatControl
  (params (Stat%20To%20Mod :type EStats%20Enum :default "NewEnumerator0") (Adj%20Value :type Float%20%28single-precision%29))
  (bind _control_max (Variables|Default|GetControl%20Max))
  (bind _returnvalue (Math|Conversions|ToFloat(Integer) _control_max))
  (bind _statstruct (CallFunction|FindStat Stat%20To%20Mod))
  (if (<= (+ (.Control (Utilities|Struct|BreakCharStatsV2 _statstruct)) Adj%20Value) _returnvalue)
    (Utilities|Struct|SetmembersinCharStatsV2 _statstruct (+ (.Control (Utilities|Struct|BreakCharStatsV2 _statstruct)) Adj%20Value))
    (else
      (Utilities|Struct|SetmembersinCharStatsV2 _statstruct _returnvalue)))
  (return false))

(fn IFModStatEXPGainRate
  (params (StatToAdjust :type EStats%20Enum :default "NewEnumerator0") (AmountToAdjust :type Float%20%28single-precision%29))
  (bind _maxexpmultiplier (Variables|Default|GetMaxExpMultiplier))
  (bind _statstruct (CallFunction|FindStat StatToAdjust))
  (if (and (<= (+ (.ExperienceGainRate (Utilities|Struct|BreakCharStatsV2 _statstruct)) AmountToAdjust) _maxexpmultiplier) (> (+ (.ExperienceGainRate (Utilities|Struct|BreakCharStatsV2 _statstruct)) AmountToAdjust) 0.0))
    (Utilities|Struct|SetmembersinCharStatsV2 _statstruct (+ (.ExperienceGainRate (Utilities|Struct|BreakCharStatsV2 _statstruct)) AmountToAdjust))
    (elif (> (+ (.ExperienceGainRate (Utilities|Struct|BreakCharStatsV2 _statstruct)) AmountToAdjust) 0.0)
      (Utilities|Struct|SetmembersinCharStatsV2 _statstruct _maxexpmultiplier)
      (else
        (Utilities|Struct|SetmembersinCharStatsV2 _statstruct 0.001))))
  (return false))

(fn IFModStatFocus
  (params (Stat%20To%20Mod :type EStats%20Enum :default "NewEnumerator0") (Adj%20Value :type Float%20%28single-precision%29))
  (bind _focus_max (Variables|Default|GetFocus%20Max))
  (bind _returnvalue (Math|Conversions|ToFloat(Integer) _focus_max))
  (bind _statstruct (CallFunction|FindStat Stat%20To%20Mod))
  (if (<= (+ (.Focus (Utilities|Struct|BreakCharStatsV2 _statstruct)) Adj%20Value) _returnvalue)
    (Utilities|Struct|SetmembersinCharStatsV2 _statstruct (+ (.Focus (Utilities|Struct|BreakCharStatsV2 _statstruct)) Adj%20Value))
    (else
      (Utilities|Struct|SetmembersinCharStatsV2 _statstruct _returnvalue)))
  (return false))

(fn IFModStatFreq
  (params (Stat%20To%20Mod :type EStats%20Enum :default "NewEnumerator0") (Freq%20Adj :type Float%20%28single-precision%29))
  (bind _statstruct (CallFunction|FindStat Stat%20To%20Mod))
  (if (and (<= (+ (.Amplitude (Utilities|Struct|BreakCharStatsV2 _statstruct)) Freq%20Adj) (Math|Conversions|ToFloat(Integer) (* (.Score (Utilities|Struct|BreakCharStatsV2 _statstruct)) (Variables|Default|GetFreqMultiplier)))) (> (+ (.Amplitude (Utilities|Struct|BreakCharStatsV2 _statstruct)) Freq%20Adj) 0.0))
    (Utilities|Struct|SetmembersinCharStatsV2 _statstruct (+ (.Amplitude (Utilities|Struct|BreakCharStatsV2 _statstruct)) Freq%20Adj))
    (elif (> (+ (.Amplitude (Utilities|Struct|BreakCharStatsV2 _statstruct)) Freq%20Adj) 0.0)
      (Utilities|Struct|SetmembersinCharStatsV2 _statstruct (Math|Conversions|ToFloat(Integer) (* (.Score (Utilities|Struct|BreakCharStatsV2 _statstruct)) (Variables|Default|GetFreqMultiplier))))
      (else
        (Utilities|Struct|SetmembersinCharStatsV2 _statstruct 0.25))))
  (return 0.0))

(fn IFModStatPhase
  (params (Stat%20To%20Mod :type EStats%20Enum :default "NewEnumerator0") (Phase%20Adj :type Float%20%28single-precision%29))
  (bind _statstruct (CallFunction|FindStat Stat%20To%20Mod))
  (Utilities|Struct|SetmembersinCharStatsV2 _statstruct (Math|Float|%(Float) (+ (.Phase (Utilities|Struct|BreakCharStatsV2 _statstruct)) Phase%20Adj) 3.6e+02))
  (return 0.0))

(fn IFModStatScore
  (params (Stat%20To%20Mod :type EStats%20Enum :default "NewEnumerator0") (Adj%20Value :type Integer))
  (return 0))