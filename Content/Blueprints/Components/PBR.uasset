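; PBR component that gives its owning Character a dynamic physically based material.
; On component initialization it builds an instance of PlayerMaterial from a fixed color and material type, looked up in color and material-type libraries, and applies it to the mesh's first slot.
; A helper function returns a new player material instance for a given character without setting color or type explicitly, while the static-object counterpart is an empty stub.
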(event `self.ReceiveTick`
  (params (DeltaSeconds :type "Float (single-precision)")))

(event `self.ReceiveInitializeComponent`
  (bind _ascharacter (cast `Character` (`self.GetOwner`)))
  (bind _output_material (`/Game/Blueprints/Logical_Structures/FunctionLibraries/MaterialFunctionLibrary.Create Dynamic PBR Material Instance` null (`self.player material`) "NewEnumerator1" (`self.PBR_colors`) "NewEnumerator14" (`self.PBR_material_types`)))
  (`PrimitiveComponent.SetMaterial` (`Character.Mesh` _ascharacter) 0 _output_material))

(fn `GetNewPBRPlayerMaterialInstance`
  (params (`Player Character` :type "/Game/Blueprints/CharacterBPs/MyCharacter_V2 Object Reference"))
  (returns (`PBR Material` :type "MaterialInstanceDynamic Object Reference"))
  (bind _output_material (`/Game/Blueprints/Logical_Structures/FunctionLibraries/MaterialFunctionLibrary.Create Dynamic PBR Material Instance` (`Character.Mesh` `Player Character`) (`self.player material`) "NewEnumerator0" (`self.PBR_colors`) "NewEnumerator0" (`self.PBR_material_types`)))
  (return _output_material))

(fn `GetNewPBRStaticObjectMaterialInstance`
  (params (Target :type "Actor Object Reference"))
  (returns (`PBR Material` :type "MaterialInstanceDynamic Object Reference"))
  (return null))