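; CharVitals is a character component that holds health, mana and stamina values and exposes read access to them.
; Getters return current and maximum values, and health and mana percentages are current divided by maximum as floats.
; GetFatiguePercent and all Modify functions for health, mana and fatigue are stubs returning zero, so nothing here changes the values.
; The event graph contains only disabled placeholder events.
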(event `self.ReceiveTick`
  (params (DeltaSeconds :type "Float (single-precision)")))

(event `self.ReceiveInitializeComponent`)

(fn `Get Health`
  (returns (`Current Health` :type Integer))
  (return (`self.CurHealth`)))

(fn `GetFatiguePercent`
  (returns (FatiguePercent :type "Float (double-precision)"))
  (return 0.0))

(fn `GetHealthPercent`
  (returns (HPPercent :type "Float (double-precision)"))
  (return (/ (`KismetMathLibrary.Conv_IntToDouble` (`self.CurHealth`)) (`KismetMathLibrary.Conv_IntToDouble` (`self.MaxHealth`)))))

(fn `GetMana`
  (returns (`Current Mana` :type Integer))
  (return (`self.CurMana`)))

(fn `GetManaPercent`
  (returns (MPPercent :type "Float (double-precision)"))
  (return (/ (`KismetMathLibrary.Conv_IntToDouble` (`self.CurMana`)) (`KismetMathLibrary.Conv_IntToDouble` (`self.MaxMana`)))))

(fn `GetMaxHealth`
  (returns (`Max Health` :type Integer))
  (return (`self.MaxHealth`)))

(fn `GetMaxMana`
  (returns (`Max Mana` :type Integer))
  (return (`self.MaxMana`)))

(fn `GetMaxStamina`
  (returns (`Max Stamina` :type Integer))
  (return (`self.MaxStamina`)))

(fn `GetStamina`
  (returns (`Current Stamina` :type Integer))
  (return (`self.CurStamina`)))

(fn `ModifyCharFatigue`
  (params (FatigueToAdd :type "Float (double-precision)"))
  (returns (`New Value` :type "Float (double-precision)"))
  (return 0.0))

(fn `ModifyCharHealth`
  (params (HPToAdd :type "Float (double-precision)"))
  (returns (`new Value` :type "Float (double-precision)"))
  (return 0.0))

(fn `ModifyCharMana`
  (params (MPToAdd :type "Float (double-precision)"))
  (returns (`New Value` :type "Float (double-precision)"))
  (return 0.0))

(fn `ModifyCharMaxFatigue`
  (params (FatigueToAdd :type "Float (double-precision)"))
  (returns (`New Value` :type "Float (double-precision)"))
  (return 0.0))

(fn `ModifyCharMaxHealth`
  (params (MPToAdd :type "Float (double-precision)"))
  (returns (`New Value` :type "Float (double-precision)"))
  (return 0.0))

(fn `ModifyCharMaxMana`
  (params (ManaToDec :type "Float (double-precision)"))
  (returns (`New Value` :type "Float (double-precision)"))
  (return 0.0))