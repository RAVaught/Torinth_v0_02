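; CharUI is a component that creates and manages the player's HUD widgets: game HUD, character screen, mini skill display, inventory and context menu.
; On initialization it adds the default widgets to the viewport, mostly hidden, and toggle functions switch character and inventory visibility.
; Helpers spawn menus at the mouse and fill a six-column inventory grid.
; Context menu population is unfinished: SendContextMenu's logic is disconnected and AddItemsToContextMenu only duplicates widget creation.
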(event EventTick
  (params (DeltaSeconds :type Float%20%28single-precision%29)))

(event EventInitializeComponent
  (CallFunction|CreateDefaultUI))

(fn SetSkillHud
  (Variables|/Game/Blueprints/UIBPs/UI_Hud/UI_HUD_Character_Skills_INGAME_mini.UI_HUD_Character_Skills_INGAME_mini_C|Setlast_skill_level (Variables|ScreenReferences|GetUI_HUD_IngameSkillMini) (.Level (Utilities|Struct|BreakSkillDefinition (Variables|/Game/Blueprints/GameMechanicBPs/Classes/Skills/ROOT_CharSkill.ROOT_CharSkill_C|GetSkill%20Definition (Variables|Mechanics|GetLastUsed))))))

(fn CreateContextMenuWidget
  (bind _returnvalue (Game|GetPlayerController 0))
  (bind (_locationx _locationy) (Game|Player|GetMousePosition _returnvalue))
  (bind _returnvalue_2 (UserInterface|CreateWidget "/Game/Blueprints/UIBPs/UI_Hud/UI_HUD_ContextMenu.UI_HUD_ContextMenu_C" _returnvalue))
  (Variables|ScreenReferences|SetUI_HUD_ContextMenu _returnvalue_2)
  (UserInterface|Viewport|AddtoViewport _returnvalue_2 0)
  (Class|UserWidget|SetPositioninViewport (Variables|ScreenReferences|GetUI_HUD_ContextMenu) (Math|Vector2D|MakeVector2D _locationx _locationy))
  (Variables|Mechanics|SetContextMenuActive true))

(fn AddItemstoContextMenu
  (bind _returnvalue (Game|GetPlayerController 0))
  (bind (_locationx _locationy) (Game|Player|GetMousePosition _returnvalue))
  (bind _returnvalue_2 (UserInterface|CreateWidget "/Game/Blueprints/UIBPs/UI_Hud/UI_HUD_ContextMenu.UI_HUD_ContextMenu_C" _returnvalue))
  (Variables|ScreenReferences|SetUI_HUD_ContextMenu _returnvalue_2)
  (UserInterface|Viewport|AddtoViewport _returnvalue_2 0)
  (Class|UserWidget|SetPositioninViewport (Variables|ScreenReferences|GetUI_HUD_ContextMenu) (Math|Vector2D|MakeVector2D _locationx _locationy))
  (Variables|Mechanics|SetContextMenuActive true))

(fn CreateContextButtons
  (params (ButtonInfo :type EContextMenu%20Enum :default "NewEnumerator0"))
  (bind _returnvalue (Utilities|String|EnumtoString ButtonInfo))
  (bind _returnvalue_2 (UserInterface|CreateWidget "/Game/Blueprints/UIBPs/UI_Hud/UI_HUD_CMButton.UI_HUD_CMButton_C" (Game|GetPlayerController 0)))
  (Variables|/Game/Blueprints/UIBPs/UI_Hud/UI_HUD_CMButton.UI_HUD_CMButton_C|SetTextToPrint _returnvalue_2 _returnvalue)
  ;[1 1 1] Creates Button Text
  (Rendering|Components|TextRender|SetText (Variables|/Game/Blueprints/UIBPs/UI_Hud/UI_HUD_CMButton.UI_HUD_CMButton_C|GetTextBlock_300 _returnvalue_2) (Utilities|Text|ToText(String) _returnvalue))
  ;[1 1 1] Defines which event this button will call
  (Variables|/Game/Blueprints/UIBPs/UI_Hud/UI_HUD_CMButton.UI_HUD_CMButton_C|SetCMEventToCall _returnvalue_2 "NewEnumerator0")
  ;[1 1 1] Provides a reference to the item being clicked
  (Variables|/Game/Blueprints/UIBPs/UI_Hud/UI_HUD_CMButton.UI_HUD_CMButton_C|SetObjectReference. _returnvalue_2 (Variables|Mechanics|GetTempUITarget))
  (return (Variables|/Game/Blueprints/UIBPs/UI_Hud/UI_HUD_CMButton.UI_HUD_CMButton_C|GetButton_34 _returnvalue_2)))

(fn CreateInventoryMenuWidget
  (bind _returnvalue (Game|GetPlayerController 0))
  (bind (_locationx _locationy) (Game|Player|GetMousePosition _returnvalue))
  (bind _returnvalue_2 (UserInterface|CreateWidget "/Game/Blueprints/UIBPs/UI_Hud/UI_HUD_Inventory.UI_HUD_Inventory_C" _returnvalue))
  (Variables|ScreenReferences|SetUI_HUD_Inventory _returnvalue_2)
  (UserInterface|Viewport|AddtoViewport _returnvalue_2 0)
  (Class|UserWidget|SetPositioninViewport (Variables|ScreenReferences|GetUI_HUD_Inventory) (Math|Vector2D|MakeVector2D _locationx _locationy))
  (Variables|Mechanics|SetInventoryOpen true))

(fn AddItemstoInventoryMenu
  (LocalVariables|SetTrow 0)
  (LocalVariables|SetTcol 0)
  (for _array_element (Variables|Default|GetRootInventory)
    ;[1 1 1] Create Buttons
    (Inventory|CreateInventoryButtons)
    (bind _returnvalue (Widget|Panel|AddChild (Variables|/Game/Blueprints/UIBPs/UI_Hud/UI_HUD_Inventory.UI_HUD_Inventory_C|GetInventoryGrid (Variables|ScreenReferences|GetUI_HUD_Inventory)) 0))
    ;[0.1974 1 0.207] Update Slot information for each button as it is created
    ;;[1 1 1] Set Row and Column
    (bind _asuniform_grid_slot (Utilities|Casting|CastToUniformGridSlot _returnvalue))
    (Class|UniformGridSlot|SetRow _asuniform_grid_slot (LocalVariables|GetTrow))
    (Class|UniformGridSlot|SetColumn _asuniform_grid_slot (LocalVariables|GetTcol))
    ;;[1 1 1] Increment Column
    (LocalVariables|SetTcol (+ (LocalVariables|GetTcol) 1))
    ;;[1 1 1] Create new row if needed and reset column to 0
    (if (== (LocalVariables|GetTcol) 6)
      (LocalVariables|SetTrow (+ (LocalVariables|GetTrow) 1))
      (LocalVariables|SetTcol 0))))

(fn CreateInventoryButtons
  (params (TargetObject :type Root%20Item%20Object%20Reference))
  (bind _returnvalue (UserInterface|CreateWidget "/Game/Blueprints/UIBPs/UI_Hud/UI_HUD_Inventory_slot.UI_HUD_Inventory_slot_C" (Game|GetPlayerController 0)))
  (Variables|/Game/Blueprints/UIBPs/UI_Hud/UI_HUD_Inventory_slot.UI_HUD_Inventory_slot_C|SetItemRef _returnvalue TargetObject)
  (return (Variables|/Game/Blueprints/UIBPs/UI_Hud/UI_HUD_Inventory_slot.UI_HUD_Inventory_slot_C|GetInvButton _returnvalue)))

(fn CloseWidget
  (params (Widget%20To%20Close :type Widget%20Object%20Reference))
  (Widget|RemovefromParent Widget%20To%20Close)
  (return false))

(fn CreateDefaultUI
  (bind _returnvalue (UserInterface|CreateWidget "/Game/Blueprints/UIBPs/UI_Hud/UI_HUD_Game_Loader_v2.UI_HUD_Game_Loader_v2_C"))
  (bind _output_get (Variables|ScreenReferences|SetUI_HUD_Game_Loader _returnvalue))
  (UserInterface|Viewport|AddtoViewport _output_get 0)
  (bind _returnvalue_2 (UserInterface|CreateWidget "/Game/Blueprints/UIBPs/UI_Hud/UI_HUD_Character_loader.UI_HUD_Character_loader_C"))
  (bind _output_get_2 (Variables|ScreenReferences|SetUI_HUD_CharacterLoader _returnvalue_2))
  (Widget|SetVisibility _output_get_2 "Hidden")
  (UserInterface|Viewport|AddtoViewport _output_get_2 0)
  (bind _returnvalue_3 (UserInterface|CreateWidget "/Game/Blueprints/UIBPs/UI_Hud/UI_HUD_Character_Skills_INGAME_mini.UI_HUD_Character_Skills_INGAME_mini_C"))
  (bind _output_get_3 (Variables|ScreenReferences|SetUI_HUD_IngameSkillMini _returnvalue_3))
  (Widget|SetVisibility _output_get_3 "Hidden")
  (UserInterface|Viewport|AddtoViewport _output_get_3 0)
  (bind _returnvalue_4 (UserInterface|CreateWidget "/Game/Blueprints/UIBPs/UI_Hud/UI_HUD_Inventory.UI_HUD_Inventory_C"))
  (bind _output_get_4 (Variables|ScreenReferences|SetUI_HUD_Inventory _returnvalue_4))
  (Widget|SetVisibility _output_get_4 "Hidden")
  (UserInterface|Viewport|AddtoViewport _output_get_4 0)
  (return false))

(fn SendContextMenu
  (params (MenuArray :type Array%20of%20EContextMenu%20Enums) (Target%20Object :type Actor%20Object%20Reference))
  (return false))

(fn ShowContextMenu
  (if true
    (Widget|RemovefromParent (Variables|ScreenReferences|GetUI_HUD_ContextMenu)))
  (ContextMenu|CreateContextMenuWidget)
  (ContextMenu|AddItemstoContextMenu)
  (return false))

(fn ToggleCharacterScreen
  (bind _ui_hud_characterloader (Variables|ScreenReferences|GetUI_HUD_CharacterLoader))
  ;[1 0.2207 0.3358] When C is pressed, the bool is checked, if false, the widget is displayed, if true, the widge is turned off.
  (if (Variables|Mechanics|GetCharacterScreenActive)
    (Widget|SetVisibility _ui_hud_characterloader "Hidden")
    (Variables|Mechanics|SetCharacterScreenActive false)
    (else
      (Widget|SetVisibility _ui_hud_characterloader "Visible")
      (Variables|Mechanics|SetCharacterScreenActive true)))
  (return false))

(fn ToggleInventoryScreen
  (bind _ui_hud_inventory (Variables|ScreenReferences|GetUI_HUD_Inventory))
  ;[1 1 1] Open inventory Window
  (if (Variables|Mechanics|GetInventoryOpen)
    (Widget|SetVisibility _ui_hud_inventory "Hidden")
    (Variables|Mechanics|SetInventoryOpen false)
    (else
      (Widget|SetVisibility _ui_hud_inventory "Visible")
      (Variables|Mechanics|SetInventoryOpen true)))
  (return false))