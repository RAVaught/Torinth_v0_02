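; DefaultGM is a game-mechanic Blueprint that holds a debug-mode flag and stat layout values.
; ToggleDebug uses a FlipFlop to switch DebugMode on and off with a printed message, and the construction script starts it off.
; GetStatOffset and GetStatOrder expose their stored variables, while AppendItemToItemsList is a stub that always returns false.
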(event `ToggleDebug`
  (`/Engine/EditorBlueprintResources/StandardMacros.FlipFlop`
    (:`A`
      (set `self.DebugMode` true)
      (`KismetSystemLibrary.PrintString` "Debug Mode Active"))
    (:`B`
      (set `self.DebugMode` false)
      (`KismetSystemLibrary.PrintString` "Debug Mode Disabled"))))

(fn `AppendItemToItemsList`
  (params (`Item To Add` :type "/Game/Blueprints/Data_Structures/Structs/Items/Item_Inventory_Struct Structure"))
  (returns (Return :type Boolean))
  (return false))

(fn `GetStatOffset`
  (returns (StatOffset :type "Array of Byte"))
  (return (`self.StatOffset`)))

(fn `GetStatOrder`
  (returns (StatOrder :type "Array of /Game/Blueprints/Data_Structures/Enums/MOBSpecific/EStats Enum"))
  (return (`self.StatOrder`)))

(fn `UserConstructionScript`
  (set `self.DebugMode` false))