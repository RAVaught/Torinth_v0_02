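; World clock Blueprint that tracks in-game time and calendar, along with sun and moon visibility and lunar phase.
; A looping one-second timer fires a dispatcher that increments seconds, cascading by configurable lengths into minutes, hours, days, weeks and months.
; Hour rollovers update sun and moon flags, and day rollovers update moon phase.
; IncYear is never called, and most interface getters for current time return placeholder values.
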(event `self.ReceiveBeginPlay`
  (add `self.TestClockDispatcher` self (delegate `TestClockDispatcher_Event`))
  (`KismetSystemLibrary.K2_SetTimer` self "WorldClock" 1.0 true))

(event `TestClockDispatcher_Event`
  ;[1 1 1] 1PPS & Seconds
  (set `self.curSeconds` (+ (`self.curSeconds`) 1))
  (`self.incMinutes`))

(fn `IF_GetDay`
  (returns (Days :type Integer))
  (return 0))

(fn `IF_GetDayLength`
  (returns (Length :type Integer))
  (return (`self.DayLength`)))

(fn `IF_GetDaysTotal`
  (returns (`Total Days` :type Integer))
  (return 0))

(fn `IF_GetHourLength`
  (returns (Length :type Integer))
  (return (`self.HourLength`)))

(fn `IF_GetHours`
  (returns (Hours :type Integer))
  (return 0))

(fn `IF_GetMinuteLength`
  (returns (Length :type Integer))
  (return (`self.MinuteLength`)))

(fn `IF_GetMinutes`
  (returns (Minutes :type Integer))
  (return 0))

(fn `IF_GetMonth`
  (returns (Month :type Integer) (`Month Name` :type String))
  (return 0 ""))

(fn `IF_GetMonthLength`
  (returns (Length :type Integer))
  (return (`self.MonthLength`)))

(fn `IF_GetSeconds`
  (returns (Seconds :type Integer))
  (return 0))

(fn `IF_GetWeekLength`
  (returns (Length :type Integer))
  (return 0))

(fn `IF_GetYear`
  (returns (Year :type Integer))
  (return 0))

(fn `IF_GetYearLength`
  (returns (Length :type Integer))
  (return (`self.YearLength`)))

(fn `Inc Day`
  ;[1 1 1] Days
  (if (== (mod (`self.curHour`) (`self.DayLength`)) 0)
    (set `self.curHour` 0)
    (set `self.curDay` (+ (`self.curDay`) 1))
    (set `self.TotalDays` (+ (`self.TotalDays`) 1))
    (`self.Inc Week`)
    (`self.Inc Month`)
    (`self.SetLunarPhase`)))

(fn `Inc Hour`
  ;[1 1 1] Hours
  (if (== (mod (`self.curMinute`) (`self.HourLength`)) 0)
    (set `self.curMinute` 0)
    (set `self.curHour` (+ (`self.curHour`) 1))
    ;[1 1 1] Check to see if we need to adjust the sun or moon
    (`self.SetSunVisible`)
    (`self.SetIsMoonVisible`)
    ;[1 1 1] Check to see if days need to update
    (`self.Inc Day`)))

(fn `Inc Month`
  ;[1 1 1] Check to see if weeks needs to update, and if so, increment by 1
  (if (== (mod (`self.curDay`) (`self.MonthLength`)) 0)
    (set `self.curMonth` (+ (`self.curMonth`) 1))))

(fn `Inc Week`
  ;[1 1 1] Check to see if weeks needs to update, and if so, increment by 1
  (if (== (mod (`self.curDay`) (`self.WeekLength`)) 0)
    (set `self.CurWeeks` (+ (`self.CurWeeks`) 1))))

(fn `Inc Year`
  ;[1 1 1] Year
  (if (== (mod (`self.curMonth`) (`self.YearLength`)) 0)
    (set `self.curMonth` 1)
    (set `self.curYear` (+ (`self.curYear`) 1))))

(fn `incMinutes`
  ;[1 1 1] Divide current seconds by minute length, if remainder is 0, increment minutes and clear seconds
  (if (== (mod (`self.curSeconds`) (`self.MinuteLength`)) 0)
    (set `self.curSeconds` 0)
    (set `self.curMinute` (+ (`self.curMinute`) 1))
    (`self.Inc Hour`)))

(fn `SetIsMoonVisible`
  ;[1 1 1] Check to see if the time is after moonrise
  (if (>= (`self.curHour`) (`self.MoonriseHour`))
    ;[1 1 1] If So, set the moon to visible
    (set `self.MoonVisible` true)
    (`KismetSystemLibrary.PrintString` "WorldClock Event: The moon has peeked over the horizon.")
    (else
      ;[1 1 1] If it is not, see if we need to make the moon disappear
      (if (>= (`self.curHour`) (`self.MoonsetHour`))
        (set `self.MoonVisible` false)
        (`KismetSystemLibrary.PrintString` "WorldClock Event: The moon has dipped below the horizon.")))))

(fn `SetLunarPhase`
  (if (== (mod (`self.curDay`) (/ (`self.MonthLength`) (enumcount `/Game/Blueprints/Data_Structures/Enums/GenericInfo/EMoonPhase`))) 0)
    (if (< (`KismetMathLibrary.Conv_ByteToInt` (`self.curMoonPhase`)) (enumcount `/Game/Blueprints/Data_Structures/Enums/GenericInfo/EMoonPhase`))
      (set `self.curMoonPhase` (cast `/Game/Blueprints/Data_Structures/Enums/GenericInfo/EMoonPhase` (+ (`self.curMoonPhase`) 1)))
      (else
        (set `self.curMoonPhase` "NewEnumerator0")))
    (`KismetSystemLibrary.PrintString` (`KismetStringLibrary.Concat_StrStr` "WorldClock: Moonphase updated to " (`|GetEnumeratorNameAsString` (enumliteral `/Game/Blueprints/Data_Structures/Enums/GenericInfo/EMoonPhase` (`self.curMoonPhase`)))) false)))

(fn `SetSunVisible`
  (if (`self.IsDay`)
    (if (>= (`self.curHour`) (`self.SunsetHour`))
      (set `self.IsDay` false)
      (`KismetSystemLibrary.PrintString` "WorldClock Event: The Sun has dipped below the horizon."))
    (elif (>= (`self.curHour`) (`self.SunriseHour`))
      (set `self.IsDay` true)
      (`KismetSystemLibrary.PrintString` "WorldClock Event: The Sun has peeked over the horizon."))))

(fn `UserConstructionScript`)

(fn `WorldClock`
  ;[1 1 1] 1PPS & Seconds
  (`self.TestClockDispatcher` self))